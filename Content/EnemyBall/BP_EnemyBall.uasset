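; BP_EnemyBall is an enemy ball that lunges at pawns it sees and has hit logic meant to knock back BP_BallPlayer.
; Pawn detection applies a horizontal impulse toward the pawn, scaled by Force and limited by a one-second game-time cooldown.
; Collision hits print a debug message and apply the scaled normal impulse to the player's ball, but only on the failed-cast branch, where that reference is invalid.
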(event `self.Detection.OnSeePawn`
  (params (Pawn :type "Pawn Object Reference"))
  (bind (_returnvalue_x _returnvalue_y) (`KismetMathLibrary.BreakVector` (* (`KismetMathLibrary.Normal` (- (`SceneComponent.K2_GetComponentLocation` (`Actor.RootComponent` Pawn)) (`SceneComponent.K2_GetComponentLocation` (`self.Ball`)))) (`self.Force`))))
  (`/Engine/EditorBlueprintResources/StandardMacros.CompareFloat` (`self.Cooldown`) (`KismetSystemLibrary.GetGameTimeInSeconds`)
    (:`<`
      (`PrimitiveComponent.AddImpulse` (`self.Ball`) (`KismetMathLibrary.MakeVector` _returnvalue_x _returnvalue_y) "None" false)
      (set `self.Cooldown` (+ (`KismetSystemLibrary.GetGameTimeInSeconds`) 1.0)))))

(event `self.Collision.OnComponentHit`
  (params (HitComponent :type "PrimitiveComponent Object Reference") (OtherActor :type "Actor Object Reference") (OtherComp :type "PrimitiveComponent Object Reference") (NormalImpulse :type "Vector Structure") (Hit :type "HitResult Structure (by ref)"))
  (bind _asbp_ball_player (cast `/Game/BallPlayer/BP_BallPlayer` OtherActor)
    (:`CastFailed`
      (`KismetSystemLibrary.PrintText` "Aplique fuerza")
      (`PrimitiveComponent.AddImpulse` (`/Game/BallPlayer/BP_BallPlayer.BallPlayer` _asbp_ball_player) (* NormalImpulse (`self.Impulse Strength`)) "None" false))))

(fn `UserConstructionScript`)