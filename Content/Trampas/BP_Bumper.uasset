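; BP_Bumper is a bumper trap that pushes the player's ball when it enters the trigger Box.
; On overlap it casts to BP_BallPlayer and applies an impulse to the BallPlayer component, computed as PercentileSpeed times ImpulseStrength.
; PercentileSpeed is read from a separate Player reference, which this graph never sets.
; A Bump timeline animation, marked as not working, is left disconnected and never runs.
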(event `self.Box.OnComponentBeginOverlap`
  (params (OverlappedComponent :type "PrimitiveComponent Object Reference") (OtherActor :type "Actor Object Reference") (OtherComp :type "PrimitiveComponent Object Reference") (OtherBodyIndex :type Integer) (bFromSweep :type Boolean) (SweepResult :type "HitResult Structure (by ref)"))
  ;[1 1 1] Bumper Impulse
  (bind _asbp_ball_player (cast `/Game/ThirdPerson/Blueprints/BP_BallPlayer` OtherActor))
  (`PrimitiveComponent.AddImpulse` (`/Game/ThirdPerson/Blueprints/BP_BallPlayer.BallPlayer` _asbp_ball_player) (* (`/Game/ThirdPerson/Blueprints/BP_BallPlayer.PercentileSpeed` (`self.Player`)) (`self.ImpulseStrength`)) "None" false))

(fn `UserConstructionScript`)