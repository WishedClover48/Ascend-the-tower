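; BP_Wind is a wind volume that pushes physics objects inside a box-shaped zone.
; The construction script sizes the WindZone box from the ZoneX, ZoneY and ZoneZ variables.
; Every tick it loops over the components overlapping the box and applies the WindStrength force at the world location of each one that simulates physics.
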(event `self.ReceiveTick`
  (params (DeltaSeconds :type "Float (single-precision)"))
  (for _array_element (`PrimitiveComponent.GetOverlappingComponents` (`self.WindZone`))
    (if (`SceneComponent.IsSimulatingPhysics` _array_element "None")
      (`PrimitiveComponent.AddForceAtLocation` _array_element (`self.WindStrength`) (`SceneComponent.K2_GetComponentLocation` _array_element) "None"))))

(fn `UserConstructionScript`
  (`BoxComponent.SetBoxExtent` (`self.WindZone`) (`KismetMathLibrary.MakeVector` (`self.ZoneX`) (`self.ZoneY`) (`self.ZoneZ`)) true))