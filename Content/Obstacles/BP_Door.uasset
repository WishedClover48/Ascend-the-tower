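; BP_Door is an obstacle door that opens by dissolving and closes again after a delay.
; BeginPlay creates a dynamic dissolve material on the Cube and stores it for later updates.
; OpenDoor plays a timeline that drives the dissolve parameter, then disables actor collision, prints the countdown duration and calls ClosingDoor.
; ClosingDoor waits, then restores collision and snaps the material back without animation.
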(event `self.ReceiveBeginPlay`
  ;[1 1 1] Crate Dynamic Material
  (bind _returnvalue (`PrimitiveComponent.CreateDynamicMaterialInstance` (`self.Cube`) 0 "/Game/Effects/Disolve.Disolve" "None"))
  (bind _output_get (set `self.DynamicMaterial` _returnvalue))
  (`MaterialInstanceDynamic.SetScalarParameterValue` _output_get "DisovePresent" 1.0))

(event `OpenDoor`
  (bind (_direction _newtrack_0) (`Timeline|Openning door` :!via `PlayFromStart`)
    (:`Update`
      (`MaterialInstanceDynamic.SetScalarParameterValue` (`self.DynamicMaterial`) "DisovePresent" _newtrack_0))
    (:`Finished`
      (`self.SetActorEnableCollision` false)
      (`KismetSystemLibrary.PrintText` (`KismetTextLibrary.Conv_DoubleToText` (`self.DoorRemainsOpenFor`) "HalfToEven"))
      (`KismetSystemLibrary.PrintText` "Door will close in...")
      (`self.ClosingDoor`))))

(event `ClosingDoor`
  (`KismetSystemLibrary.Delay` (`self.DoorRemainsOpenFor`))
  (`self.SetActorEnableCollision` true)
  (`MaterialInstanceDynamic.SetScalarParameterValue` (`self.DynamicMaterial`) "DisovePresent" 1.0))

(fn `UserConstructionScript`)