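; BP_InteractableObject is a trigger obstacle that opens its TargetDoor and prints a message when a BP_BallPlayer overlaps its Sphere.
; Activation plays a timeline that animates the Torus Z scale.
; That timeline's Update also feeds a delay of the door's DoorRemainsOpenFor, leading to ResetActivator.
; After a further short delay, ResetActivator plays a second timeline in reverse to animate the Torus back.
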(event `self.Sphere.OnComponentBeginOverlap`
  (params (OverlappedComponent :type "PrimitiveComponent Object Reference") (OtherActor :type "Actor Object Reference") (OtherComp :type "PrimitiveComponent Object Reference") (OtherBodyIndex :type Integer) (bFromSweep :type Boolean) (SweepResult :type "HitResult Structure (by ref)"))
  (cast `/Game/BallPlayer/BP_BallPlayer` OtherActor)
  (`/Game/Obstacles/BP_Door.OpenDoor` (`self.TargetDoor`))
  (`KismetSystemLibrary.PrintText` "A door opens!")
  (`self.Activated`))

(event `Activated`
  ;[1 1 1] Animation when Activated
  (bind (_direction _newtrack_0) (`Timeline|Timeline`)
    (:`Update`
      (`SceneComponent.SetRelativeScale3D` (`self.Torus`) (`KismetMathLibrary.MakeVector` 1.5 1.5 _newtrack_0))
      (`KismetSystemLibrary.Delay` (`/Game/Obstacles/BP_Door.DoorRemainsOpenFor` (`self.TargetDoor`)))
      (`self.Reset Activator`))))

(event `Reset Activator`
  (`KismetSystemLibrary.Delay` 3.0)
  (bind (_direction _newtrack_0) (`Timeline|Timeline_0` :!via `ReverseFromEnd`)
    (:`Update`
      (`SceneComponent.SetRelativeScale3D` (`self.Torus`) (`KismetMathLibrary.MakeVector` 1.5 1.5 _newtrack_0)))))

(fn `UserConstructionScript`)